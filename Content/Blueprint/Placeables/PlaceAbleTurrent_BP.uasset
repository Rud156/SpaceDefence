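; Placeable turret that tracks the nearest sensed BaseEnemy.
; AI perception adds enemies to DetectedActors when sensed and removes them when lost.
; Each tick it selects the closest one and snaps the turret top's rotation toward it, aiming from the BulletSpawner socket.
; BeginPlay starts a looping timer that calls Fire by name, a function not defined in this graph.
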(event OnTargetPerceptionUpdated(AIPerception)
  (params (Actor :type Actor%20Object%20Reference) (Stimulus :type AI%20Stimulus%20Structure))
  (bind _asbase_enemy (Utilities|Casting|CastToBaseEnemy Actor))
  (if (.bSuccessfullySensed (Utilities|Struct|BreakAIStimulus Stimulus))
    (Utilities|Array|AddUnique (Variables|Default|GetDetected%20Actors) _asbase_enemy)
    (else
      (Utilities|Array|RemoveItem (Variables|Default|GetDetected%20Actors) _asbase_enemy))))

(event EventTick
  (params (DeltaSeconds :type Float%20%28single-precision%29))
  (bind _closest_actor (Variables|Default|GetClosest%20Actor))
  (CallFunction|SetClosestActor)
  (Utilities|IsValid _closest_actor
    (:Is%20Valid
      (Transformation|SetWorldRotation (Variables|Default|GetPivotFixTurrentTop) (Math|Rotator|FindLookatRotation (Transformation|GetSocketLocation (Variables|Default|GetPivotFixTurrentTop) "BulletSpawner") (Transformation|GetActorLocation _closest_actor)) false false))))

(event EventBeginPlay
  (Variables|Default|SetTurret (Variables|Default|GetPivotFixTurrentTop))
  (Utilities|Time|SetTimerbyFunctionName self "Fire" 0.5 true))

(fn ConstructionScript)

(fn SetClosestActor
  (LocalVariables|SetCurrent%20Closest%20Distance 99999.0)
  (Variables|Default|SetClosest%20Actor 0)
  (for _array_element (Variables|Default|GetDetected%20Actors)
    (if (< (Math|Vector|Distance(Vector) (Transformation|GetActorLocation _array_element) (Transformation|GetActorLocation)) (LocalVariables|GetCurrent%20Closest%20Distance))
      (LocalVariables|SetCurrent%20Closest%20Distance (Math|Vector|Distance(Vector) (Transformation|GetActorLocation _array_element) (Transformation|GetActorLocation)))
      (Variables|Default|SetClosest%20Actor _array_element))))