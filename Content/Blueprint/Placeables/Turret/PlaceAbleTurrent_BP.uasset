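; Placeable turret Blueprint with helper logic for targeting enemies.
; Its range check tests whether the ClosestTarget mesh lies within a fixed distance of the turret's root mesh.
; A disconnected graph in the Test function would pick the nearest BaseEnemy from sight-perceived actors, but it never runs, leaving Test empty.
; Nothing shown here assigns ClosestTarget or fires at it.
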(fn ConstructionScript)

(fn Test)

(fn CheckwithinRange
  (return (> 5e+02 (Math|Vector|Distance(Vector) (Transformation|GetWorldLocation (Variables|Default|GetRootMeshComponent)) (Transformation|GetWorldLocation (Variables|/Script/Engine.Character|GetMesh (Variables|Default|GetClosestTarget)))))))