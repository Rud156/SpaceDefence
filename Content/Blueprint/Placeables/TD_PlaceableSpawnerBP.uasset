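; Placeable spawner Blueprint with a Ghost mesh component that tracks whether its current position is colliding and resting on ground.
; Ghost overlap begin and end events set and clear IsColliding, with no count of simultaneous overlaps.
; While Ghost has a valid mesh, Tick traces 10 units down on the Visibility channel to update IsOnGround.
; The file only maintains these flags and contains no spawning or placement logic.
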(event OnComponentBeginOverlap(Ghost)
  (params (OverlappedComponent :type Primitive%20Component%20Object%20Reference) (OtherActor :type Actor%20Object%20Reference) (OtherComp :type Primitive%20Component%20Object%20Reference) (OtherBodyIndex :type Integer) (bFromSweep :type Boolean) (SweepResult :type Hit%20Result%20Structure%20%28by%20ref%29))
  (Variables|Default|SetbIsColliding true))

(event OnComponentEndOverlap(Ghost)
  (params (OverlappedComponent :type Primitive%20Component%20Object%20Reference) (OtherActor :type Actor%20Object%20Reference) (OtherComp :type Primitive%20Component%20Object%20Reference) (OtherBodyIndex :type Integer))
  (Variables|Default|SetbIsColliding false))

(event Collision|EventActorBeginOverlap
  (params (OtherActor :type Actor%20Object%20Reference)))

(event EventTick
  (params (DeltaSeconds :type Float%20%28single-precision%29))
  (bind _ghost (Variables|Default|GetGhost))
  (bind _returnvalue (Transformation|GetWorldLocation _ghost))
  (bind (_x _y _z) (Math|Vector|BreakVector _returnvalue))
  (Utilities|IsValid (Variables|/Script/Engine.StaticMeshComponent|GetStaticMesh _ghost)
    (:Is%20Valid
      (bind _outhit (Collision|LineTraceByChannel (Math|Vector|MakeVector _x _y _z) (+ _returnvalue (Math|Vector|MakeVector 0.0 0.0 -1e+01)) "TraceTypeQuery1" false 0 "None"))
      (Variables|Default|SetbIsOnGround (.bblockinghit _outhit)))))

(fn ConstructionScript)