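; BP_FPPlayer is the first-person player character, combining movement feedback with tower-defense building controls.
; Tick toggles run camera shake and interpolates trace-based foot and hip IK offsets, while events handle jump montages, crosshair and health logging.
; Input drives inventory, quick-slot ghost spawning and placement, upgrade and removal through the HUD, and wave spawning.
; Ghost snapping, rotation, interaction tracing and setup of GameMode and spawner references sit in disconnected nodes.
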(event Custom|Event%20Health%20Changed
  (params (NewHealth :type Integer))
  (Development|PrintString (Utilities|String|Append "Player Health: " (Utilities|String|ToString(Integer) NewHealth))))

(event EventMovementStatePushed
  (params (playerMovementState :type EPlayerMovementState%20Enum :default "None")))

(event EventBeginPlay
  (Utilities|FlowControl|Sequence
    (:then_0
      (bind _returnvalue (Game|SpawnActorfromClass "/Game/Blueprint/Managers/BP_InteractionDisplayManager.BP_InteractionDisplayManager_C" (Math|Transform|MakeTransform "0, 0, 0") "Undefined" 0 0))
      (Variables|Default|SetInteractionDisplayManager _returnvalue))
    (:then_1
      (bind _returnvalue_2 (UserInterface|CreateWidget "/Game/Blueprint/UI/Player/HUD_PlayerCrossHair.HUD_PlayerCrossHair_C" (Game|GetPlayerController 0)))
      (bind _output_get (Variables|Default|SetHUD_PlayerCrosshair _returnvalue_2))
      (UserInterface|Viewport|AddtoViewport _output_get 0)
      (EventDispatchers|BindEventtoOnHealthChanged (Variables|Default|GetHealthAndDamage) (delegate Custom|Event%20Health%20Changed)))))

(event EventPlayerRunJumped
  (Animation|Montage|PlayMontage (Variables|Character|GetMesh) "/Game/Blueprint/Player/Animation/BP_PlayerJumpMontage.BP_PlayerJumpMontage" 1.0 0.0 "RunJump"))

(event EventPlayerJumped
  (Animation|Montage|PlayMontage (Variables|Character|GetMesh) "/Game/Blueprint/Player/Animation/BP_PlayerJumpMontage.BP_PlayerJumpMontage" 1.0 0.0 "Jump"))

(event EventWeaponShotCameraShake
  (params (CameraShake :type Matinee%20Camera%20Shake%20Class%20Reference))
  (CameraShakes|StartCameraShake (Game|GetPlayerCameraManager 0) CameraShake 1.0 "CameraLocal" "0, 0, 0"))

(event EventTick
  (params (DeltaSeconds :type Float%20%28single-precision%29))
  (Utilities|FlowControl|Sequence
    (:then_0
      (if (Math|Boolean|NotEqual(Boolean) (Variables|Default|GetLast%20Run%20State) (Class|FPPlayer|IsRunning))
        (if (Class|FPPlayer|IsRunning)
          (bind _returnvalue (CameraShakes|StartCameraShake (Game|GetPlayerCameraManager 0) "/Game/Blueprint/Player/Camera/BP_PlayerRunCS.BP_PlayerRunCS_C" 1.0 "CameraLocal" "0, 0, 0"))
          (Variables|Default|SetRun%20Camera%20Shake _returnvalue)
          (else
            (CameraShakes|StopCameraShake (Game|GetPlayerCameraManager 0) (Variables|Default|GetRun%20Camera%20Shake) true)))))
    (:then_1
      (Variables|Default|SetLast%20Run%20State (Class|FPPlayer|IsRunning)))
    (:then_2
      (bind (_outhitlocation _foottraceoffset) (Class|FPPlayer|IKFootTrace "LeftFootSocket" (/ (Components|Capsule|GetUnscaledCapsuleHalfHeight (Variables|Default|GetCapsuleComponent)) 2.0)))
      (Variables|Character|IK|SetLeft%20Foot%20IK%20Offset (Math|Interpolation|FInterpTo (Variables|Character|IK|GetLeft%20Foot%20IK%20Offset) _foottraceoffset (Utilities|Time|GetWorldDeltaSeconds) 2e+01))
      (bind (_outhitlocation_2 _foottraceoffset_2) (Class|FPPlayer|IKFootTrace "RightFootSocket" (/ (Components|Capsule|GetUnscaledCapsuleHalfHeight (Variables|Default|GetCapsuleComponent)) 2.0)))
      (Variables|Character|IK|SetRight%20Foot%20IK%20Offset (Math|Interpolation|FInterpTo (Variables|Character|IK|GetRight%20Foot%20IK%20Offset) _foottraceoffset_2 (Utilities|Time|GetWorldDeltaSeconds) 2e+01))
      (Variables|Default|SetIkHipOffset (Math|Interpolation|FInterpTo (Variables|Default|GetIkHipOffset) (Math|Float|SelectFloat (* (Math|Float|Absolute(Float) (.z (- _outhitlocation_2 _outhitlocation))) -0.5) 0.0 (< (Math|Float|Absolute(Float) (.z (- _outhitlocation_2 _outhitlocation))) 2e+01)) (Utilities|Time|GetWorldDeltaSeconds) 2e+01)))))

(event Input|ActionEvents|InputActionPlaceNewObject
  (params (Key :type Key%20Structure :default "None"))
  (:Pressed
    (if (Variables|Default|GetBuildingFlag)
      (Variables|Default|SetBuildingFlag false)
      (bind _astd_placeable_spawner_actor (Utilities|Casting|CastToTD_PlaceableSpawnerActor (Variables|/Script/Engine.ChildActorComponent|GetChildActor (Variables|Default|GetNewSpawner))))
      (Class|TDPlaceableSpawnerActor|SpawnActorfromGhost _astd_placeable_spawner_actor (Variables|Default|GetCurrentPlaceAbleID))
      (else
        (bind _out_hit_location (Utilities|GetPlaceableHitLocationfromCamera))
        (bind _returnvalue (Class|TDPlaceableSpawnerActor|SpawnPlaceAbleGhost (Variables|Default|GetPlaceAbleSpawnerActorRef) _out_hit_location (Variables|Default|GetCurrentPlaceAbleID)))
        (Variables|Default|SetBuildingFlag _returnvalue)))))

(event Input|ActionEvents|InputActionToggleInventory
  (params (Key :type Key%20Structure :default "None"))
  (bind _gamemoderef (Variables|Default|GetGameModeRef))
  (:Pressed
    (bind _asinventory_ui_bp (Utilities|Casting|CastToInventoryUI_BP (Variables|/Script/SpaceDefence.TD_GameModeFPS|GetInventoryBPRef _gamemoderef)))
    (Default|ToggleInventory _asinventory_ui_bp)
    (Class|TDMainHUD|ToggleQuickSlotPosition (Variables|/Script/SpaceDefence.TD_GameModeFPS|GetMainHUDRef _gamemoderef))))

(event Input|ActionEvents|InputActionQuickSlot9
  (params (Key :type Key%20Structure :default "None"))
  (:Pressed
    (Utilities|SetCurrentPlaceAbleID 8)))

(event Input|ActionEvents|InputActionUpgradeObjects
  (params (Key :type Key%20Structure :default "None"))
  (:Pressed
    (Class|TDMainHUD|HandleUpgrade (Variables|/Script/SpaceDefence.TD_GameModeFPS|GetMainHUDRef (Variables|Default|GetGameModeRef)))))

(event Input|ActionEvents|InputActionRemoveObjects
  (params (Key :type Key%20Structure :default "None"))
  (:Pressed
    (Class|TDMainHUD|HandleRemoval (Variables|/Script/SpaceDefence.TD_GameModeFPS|GetMainHUDRef (Variables|Default|GetGameModeRef)))))

(event Input|ActionEvents|InputActionQuickSlot1
  (params (Key :type Key%20Structure :default "None"))
  (:Pressed
    (Utilities|SetCurrentPlaceAbleID)))

(event Input|ActionEvents|InputActionQuickSlot2
  (params (Key :type Key%20Structure :default "None"))
  (:Pressed
    (Utilities|SetCurrentPlaceAbleID 1)))

(event Input|ActionEvents|InputActionQuickSlot3
  (params (Key :type Key%20Structure :default "None"))
  (:Pressed
    (Utilities|SetCurrentPlaceAbleID 2)))

(event Input|ActionEvents|InputActionQuickSlot5
  (params (Key :type Key%20Structure :default "None"))
  (:Pressed
    (Utilities|SetCurrentPlaceAbleID 4)))

(event Input|ActionEvents|InputActionQuickSlot4
  (params (Key :type Key%20Structure :default "None"))
  (:Pressed
    (Utilities|SetCurrentPlaceAbleID 3)))

(event Input|ActionEvents|InputActionQuickSlot6
  (params (Key :type Key%20Structure :default "None"))
  (:Pressed
    (Utilities|SetCurrentPlaceAbleID 5)))

(event Input|ActionEvents|InputActionQuickSlot7
  (params (Key :type Key%20Structure :default "None"))
  (:Pressed
    (Utilities|SetCurrentPlaceAbleID 6)))

(event Input|ActionEvents|InputActionQuickSlot8
  (params (Key :type Key%20Structure :default "None"))
  (:Pressed
    (Utilities|SetCurrentPlaceAbleID 7)))

(event Input|KeyboardEvents|P
  (params (Key :type Key%20Structure :default "None"))
  (:Pressed
    (bind _astd_game_mode_fps_bp (Utilities|Casting|CastToTD_GameModeFPS_BP (Game|GetGameMode)))
    (Class|TDWaveController|SpawnWave (Variables|/Script/SpaceDefence.TD_GameModeFPS|GetWaveControllerRef _astd_game_mode_fps_bp))))

(fn ConstructionScript)

(fn CheckLeft)

(fn CheckRight)

(fn GetHitSideFunction
  (params (AxisY :type Vector) (AxisZ :type Vector) (HitNormal :type Vector)))