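; Game mode for a first-person tower defense game that sets up UI and core managers on BeginPlay.
; It creates the inventory and main HUD widgets for the first player and adds both to the viewport.
; It then spawns the currency manager, looks up the level's wave controller and map center actor, and stores references to all of them.
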(event EventBeginPlay
  (bind _returnvalue (Game|GetPlayerController 0))
  (Utilities|FlowControl|Sequence
    (:then_0
      (bind _returnvalue_2 (UserInterface|CreateWidget "/Game/Blueprint/UI/InventoryUI_BP.InventoryUI_BP_C" _returnvalue))
      (Variables|Default|SetInventoryBPRef _returnvalue_2)
      (UserInterface|Viewport|AddtoViewport _returnvalue_2 0))
    (:then_1
      (bind _returnvalue_3 (UserInterface|CreateWidget "/Game/Blueprint/UI/MainHUD.MainHUD_C" _returnvalue))
      (bind _output_get (Variables|Default|SetMainHUDRef _returnvalue_3))
      (UserInterface|Viewport|AddtoViewport _output_get 0))
    (:then_2
      (bind _returnvalue_4 (Game|SpawnActorfromClass "/Game/Blueprint/CurrencyManager/CurrencyManager_BP.CurrencyManager_BP_C" (Math|Transform|MakeTransform "0, 0, 0" "0, 0, 0" "1,1,1") "Undefined" 0 0))
      (Variables|Default|SetCurrencyManagerRef _returnvalue_4))
    (:then_3
      (bind _outactors (Actor|GetAllActorsOfClass "/Game/Blueprint/WaveSystem/WaveController_BP.WaveController_BP_C"))
      (Utilities|IsValid (Utilities|Array|Get(acopy) _outactors)
        (:Is%20Valid
          (Variables|Default|SetWaveControllerRef (Utilities|Array|Get(acopy) _outactors)))))
    (:then_4
      (bind _returnvalue_5 (Actor|GetActorOfClass "/Game/Blueprint/WaveSystem/MapCenter.MapCenter_C"))
      (Variables|Default|SetMapCenter _returnvalue_5))))

(event EventTick
  (params (DeltaSeconds :type Float%20%28single-precision%29)))

(fn ConstructionScript)