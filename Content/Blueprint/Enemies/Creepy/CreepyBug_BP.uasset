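; CreepyBug_BP is a creepy bug enemy character that uses AI perception to track tower-defense placeable actors as potential targets.
; Sensed placeables are added uniquely to a targetable-items list and removed when sensing is lost.
; Animation budgeting is enabled on BeginPlay.
; Animation Sharing registration and a velocity-based animation state selection remain in the graph but are disconnected and never run.
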(event OnTargetPerceptionUpdated(AIPerception)
  (params (Actor :type Actor%20Object%20Reference) (Stimulus :type AI%20Stimulus%20Structure))
  (bind _listofcurrenttargetableitems (Variables|Default|GetListOfCurrentTargetAbleItems))
  (bind _astd_placeables_actors (Utilities|Casting|CastToTD_PlaceablesActors Actor))
  (if (.bsuccessfullysensed Stimulus)
    (Utilities|Array|AddUnique _listofcurrenttargetableitems _astd_placeables_actors)
    (else
      (Utilities|Array|RemoveItem _listofcurrenttargetableitems _astd_placeables_actors))))

(event EventTick
  (params (DeltaSeconds :type Float%20%28single-precision%29)))

(event EventBeginPlay
  (Class|AnimationBudgetBlueprintLibrary|EnableAnimationBudget true))

(fn ConstructionScript)