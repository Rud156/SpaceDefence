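; Behavior tree service that drives the Mutant enemy's state switches through the blackboard.
; On activation it seeds TeleportCount with a random value from the pawn's min/max range.
; Each tick it moves IdleWander to Attack once that count is used up, and Attack to Wait when an attack ends.
; It detects the attack's end by comparing the pawn against the previous tick's IsAttacking key, then updates that key.
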(event EventReceiveActivationAI
  (params (OwnerController :type AI%20Controller%20Object%20Reference) (ControlledPawn :type Pawn%20Object%20Reference))
  (bind _asmutant_enemy (Utilities|Casting|CastToMutantEnemy ControlledPawn))
  (Class|BlackboardComponent|SetValueasInt (AI|GetBlackboard OwnerController) (Variables|Default|GetTeleportCount) (Math|Random|RandomIntegerinRange (Variables|/Script/SpaceDefence.MutantEnemy|GetTeleportCountMin _asmutant_enemy) (Variables|/Script/SpaceDefence.MutantEnemy|GetTeleportCountMax _asmutant_enemy))))

(event EventReceiveTickAI
  (params (OwnerController :type AI%20Controller%20Object%20Reference) (ControlledPawn :type Pawn%20Object%20Reference) (DeltaSeconds :type Float%20%28single-precision%29))
  (bind _returnvalue (AI|GetBlackboard OwnerController))
  (Utilities|FlowControl|Sequence
    (:then_0
      (if (and (<= (Class|BlackboardComponent|GetValueasInt _returnvalue (Variables|Default|GetTeleportCount)) 0) (Utilities|Enum|Equal(Enum) (Utilities|Enum|ByteToEnumEMutantState (Class|BlackboardComponent|GetValueasEnum _returnvalue (Variables|Default|GetEnemyState))) "IdleWander"))
        (AI|Components|Blackboard|SetValueasEnum _returnvalue (Variables|Default|GetEnemyState) (Utilities|Enum|LiteralenumEMutantState "Attack"))))
    (:then_1
      (bind _asmutant_enemy (Utilities|Casting|CastToMutantEnemy ControlledPawn))
      (if (Math|Boolean|ANDBoolean (ScalableFloat|GetValueasBool _returnvalue (Variables|Default|GetIsAttacking)) (not (Class|MutantEnemy|GetIsAttacking _asmutant_enemy)) (Utilities|Enum|Equal(Enum) (Utilities|Enum|ByteToEnumEMutantState (Class|BlackboardComponent|GetValueasEnum _returnvalue (Variables|Default|GetEnemyState))) "Attack"))
        (AI|Components|Blackboard|SetValueasEnum _returnvalue (Variables|Default|GetEnemyState) (Utilities|Enum|LiteralenumEMutantState "Wait"))))
    (:then_2
      (bind _asmutant_enemy_2 (Utilities|Casting|CastToMutantEnemy ControlledPawn))
      (AI|Components|Blackboard|SetValueasBool _returnvalue (Variables|Default|GetIsAttacking) (Class|MutantEnemy|GetIsAttacking _asmutant_enemy_2)))))