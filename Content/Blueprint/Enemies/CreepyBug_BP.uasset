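; Creepy bug enemy Blueprint built for cheap animation through animation budgeting and the Animation Sharing plugin.
; On BeginPlay it enables the animation budget, then after a short delay registers itself with the Animation Sharing Manager using the creepy skeleton.
; Tick sorts movement speed into three AnimState tiers.
; A disconnected loop of forward line traces never runs.
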(event EventTick
  (params (DeltaSeconds :type Float%20%28single-precision%29))
  (bind _charactermovement (Variables|Character|GetCharacterMovement))
  (bind _velocity (Variables|/Script/Engine.MovementComponent|GetVelocity _charactermovement))
  (bind _returnvalue (Math|Vector|VectorLength _velocity))
  (if (> _returnvalue 1.4e+02)
    (if (> _returnvalue 3.9e+02)
      (Variables|Default|SetAnimState "NewEnumerator2")
      (else
        (Variables|Default|SetAnimState "NewEnumerator1")))
    (else
      (Variables|Default|SetAnimState "NewEnumerator0"))))

(event EventBeginPlay
  (Class|AnimationBudgetBlueprintLibrary|EnableAnimationBudget true)
  (Utilities|FlowControl|Delay 0.2)
  (bind _returnvalue (Class|AnimationSharingManager|GetAnimationSharingManager))
  (Class|AnimationSharingManager|RegisterActorwithSkeletonBP _returnvalue self "/Game/Creatures_Pack/Mesh/SK_Creepy_Skeleton.SK_Creepy_Skeleton"))

(fn ConstructionScript)