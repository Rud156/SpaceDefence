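; Manager actor that owns the on-screen interaction progress bar for world interactions.
; On BeginPlay it creates a HUD_WorldInteraction widget for player controller 0, adds it to the viewport and starts it hidden.
; Its show, hide and set-progress events forward directly to that widget, acting as a thin wrapper around the bar.
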(event EventShowInteractionBar
  (Default|ShowBar (Variables|Default|GetHUD_InteractionBar)))

(event EventHideInteractionBar
  (Default|HideBar (Variables|Default|GetHUD_InteractionBar)))

(event EventSetInteractionBarProgress
  (params (progress :type Float%20%28single-precision%29))
  (Default|SetProgressValue (Variables|Default|GetHUD_InteractionBar) progress))

(event EventBeginPlay
  (bind _returnvalue (UserInterface|CreateWidget "/Game/Blueprint/UI/Player/HUD_WorldInteraction.HUD_WorldInteraction_C" (Game|GetPlayerController 0)))
  (bind _output_get (Variables|Default|SetHUD_InteractionBar _returnvalue))
  (UserInterface|Viewport|AddtoViewport _output_get 0)
  (Default|HideBar (Variables|Default|GetHUD_InteractionBar)))

(fn ConstructionScript)